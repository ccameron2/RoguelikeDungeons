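; Enemy character that roams the navmesh and chases the player once detected, with a widget health bar.
; Pawn sensing or overlapping the player latches IsSeeingPlayer, which is never cleared here.
; Tick syncs the bar's health, toggles it by PlayerVisibility, halts movement when Dead, and otherwise selects chase or roam.
; Both behaviours use AI MoveTo, with roaming picking a new nearby random point after each successful arrival.
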(event `self.ReceiveBeginPlay`
  (bind _aswbp_enemy_health_bar (cast `/Game/HUD/WBP_EnemyHealthBar` (`WidgetComponent.GetUserWidgetObject` (`self.HealthBar`))))
  (set `/Game/HUD/WBP_EnemyHealthBar.Health` (`self.HealthPoints`) _aswbp_enemy_health_bar)
  (set `/Game/HUD/WBP_EnemyHealthBar.MaxHealth` (`self.MaxHealth`) _aswbp_enemy_health_bar))

(event `self.ReceiveTick`
  (params (DeltaSeconds :type "Float (single-precision)"))
  (set `/Game/HUD/WBP_EnemyHealthBar.Health` (`self.HealthPoints`) (stale `self.ReceiveBeginPlay` _aswbp_enemy_health_bar))
  (if (`self.PlayerVisibility`)
    (`Widget.SetVisibility` (stale `self.ReceiveBeginPlay` _aswbp_enemy_health_bar) "Visible")
    (else
      (`Widget.SetVisibility` (stale `self.ReceiveBeginPlay` _aswbp_enemy_health_bar) "Hidden")))
  (if (`self.Dead`)
    (`MovementComponent.StopMovementImmediately` (`self.CharacterMovement`))
    (elif (`self.IsSeeingPlayer`)
      (`self.FollowPlayer`)
      (else
        (`self.RandomRoam`)))))

(event `self.ReceiveActorBeginOverlap`
  (params (OtherActor :type "Actor Object Reference"))
  (if (== OtherActor "/Game/BP_ThirdPersonCharacter.BP_ThirdPersonCharacter")
    (set `self.IsSeeingPlayer` true)))

(event `self.PawnSensing.OnSeePawn`
  (params (Pawn :type "Pawn Object Reference"))
  (set `self.IsSeeingPlayer` true))

(event `FollowPlayer`
  (if (`self.IsSeeingPlayer`)
    (`|AIMoveTo` self (0.0 0.0 0.0) (`GameplayStatics.GetPlayerCharacter` 0) 80.0)))

(event `RandomRoam`
  (if (`self.RandomPointGenerated`)
    (`|AIMoveTo` self (stale _randomlocation) null 50.0
      (:`OnSuccess`
        (set `self.RandomPointGenerated` false)))
    (else
      (bind _randomlocation (`NavigationSystemV1.K2_GetRandomLocationInNavigableRadius` (`self.K2_GetActorLocation`) 500.0 null null))
      (set `self.RandomPointGenerated` true))))

(fn `UserConstructionScript`)